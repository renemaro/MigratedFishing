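; Flying scanner probe that catches BP_EasyFish actors by scanning them, announcing itself to all fish shortly after spawn.
; MoveHere starts a looping timer that steers it toward a target until StopMoving clears it.
; A second looping timer finds the nearest fish and drains its ScanVolume faster at closer range, updating the player's fish bar.
; An emptied fish is killed and reported to the player with placeholder ID and random weight.
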(event Custom|ScannerActive
  (bind _returnvalue (Utilities|Time|SetTimerbyEvent (delegate Custom|Scanning) 0.01 true))
  (Variables|Default|SetScanningHandler _returnvalue))

(event Custom|ScanningModeON
  (bind _returnvalue (Utilities|Time|SetTimerbyEvent (delegate Custom|IsMoving) 0.01 true))
  (Variables|Default|SetMoovingTimerHandler _returnvalue))

(event Custom|IsMoving
  (Pawn|Input|AddMovementInput (Math|Vector|GetUnitDirection(Vector) (Transformation|GetActorLocation) (Variables|Default|GetTragetLocation)) (Variables|Default|GetProbeSpeed) false))

(event Custom|Scanning
  (bind (_fishref _distance) (CallFunction|ScanforFish))
  (bind _caught (CallFunction|ScanningPercentage _fishref _distance))
  (if _caught
    (Default|KillFish _fishref)
    ;[1 0.7554 0.0498] Super TEMP - need to add fish parametres
    (Class|INTPlayer|FishCaught(Message) (Game|GetPlayerCharacter 0) "Blue_Small_Fish" (Math|Random|RandomFloatinRange 3.0 1e+01))))

(event EventMoveHere
  (params (MovementLocation :type Vector :default "0, 0, 0"))
  (Variables|Default|SetTragetLocation MovementLocation)
  (CallFunction|ScanningModeON))

(event EventStopMoving
  (Utilities|Time|ClearandInvalidateTimerbyHandle (Variables|Default|GetMoovingTimerHandler)))

(event EventBeginPlay
  (Pawn|Components|CharacterMovement|SetMovementMode (Variables|Character|GetCharacterMovement) "MOVE_Flying" 0)
  (Utilities|FlowControl|Delay 1.0)
  (bind _outactors (Actor|GetAllActorsOfClass "/Game/BP/BP_EasyFish.BP_EasyFish_C"))
  (for _array_element _outactors
    (Class|INTFish|ProbeIsActive(Message) _array_element self))
  (CallFunction|ScannerActive))

(fn ConstructionScript)

(fn ScanforFish
  (bind _outactors (Actor|GetAllActorsOfClass "/Game/BP/BP_EasyFish.BP_EasyFish_C"))
  (for _array_element _outactors
    (if (< (Math|Vector|VectorLength (- (Transformation|GetActorLocation _array_element) (Transformation|GetActorLocation))) (LocalVariables|GetNearestDist%28local%29))
      (LocalVariables|SetNearestDist%28local%29 (Math|Vector|VectorLength (- (Transformation|GetActorLocation _array_element) (Transformation|GetActorLocation))))
      (LocalVariables|SetActorsList%28local%29 _array_element)))
  (return (LocalVariables|GetActorsList%28local%29) (LocalVariables|GetNearestDist%28local%29)))

(fn ScanningPercentage
  (params (FishRef :type BP%20Easy%20Fish%20Object%20Reference) (Distanse :type Float%20%28double-precision%29))
  (bind _maxscaningdistance (Variables|Default|GetMAXScaningDistance))
  (if (and (Utilities|IsValid FishRef) (< Distanse _maxscaningdistance))
    (bind _output_get (Variables|/Game/BP/BP_EasyFish.BP_EasyFish_C|SetScanVolume FishRef (- (Variables|/Game/BP/BP_EasyFish.BP_EasyFish_C|GetScanVolume FishRef) (- 1.0 (/ Distanse _maxscaningdistance)))))
    (if (<= _output_get 0.0)
      (return true)
      (else
        (Class|INTPlayer|UpdateFishBar(Message) (Game|GetPlayerCharacter 0) (- 1.0 (/ _output_get (Variables|/Game/BP/BP_EasyFish.BP_EasyFish_C|GetScanVolumeMAX FishRef))))
        (return false)))
    (else
      (return false))))