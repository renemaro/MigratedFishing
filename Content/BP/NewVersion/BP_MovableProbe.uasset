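; BP_MovableProbe is a flying character probe that travels toward a given location to scan and catch fish.
; MoveHere starts looping timers that drive movement input and measure distance to the first BP_Fish found.
; ScanTarget shows that distance on camera-facing text, colored by range, and repeatedly applies damage while in range.
; Overlapping an actor tagged Fish calls CaughtFish on it and destroys the probe.
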(event OnComponentBeginOverlap(Capsule)
  (params (OverlappedComponent :type Primitive%20Component%20Object%20Reference) (OtherActor :type Actor%20Object%20Reference) (OtherComp :type Primitive%20Component%20Object%20Reference) (OtherBodyIndex :type Integer) (bFromSweep :type Boolean) (SweepResult :type Hit%20Result%20Structure%20%28by%20ref%29))
  (if (Actor|ActorHasTag OtherActor "Fish")
    (bind _asbp_fish (Utilities|Casting|CastToBP_Fish OtherActor))
    (Default|CaughtFish _asbp_fish)
    (Actor|DestroyActor self)))

(event Custom|TryToAnalise
  (bind _returnvalue (Actor|GetActorOfClass "/Game/BP/NewVersion/BP_Fish.BP_Fish_C"))
  (Variables|Default|SetTargetFish _returnvalue)
  (bind _returnvalue_2 (Utilities|Time|SetTimerbyEvent (delegate Custom|ScanTheFish) 0.01 true))
  (Variables|Default|SetScaningTimerHandle _returnvalue_2))

(event Custom|StartMoving
  (bind _returnvalue (Utilities|Time|SetTimerbyEvent (delegate Custom|IsMoving) 0.01 true))
  (Variables|Default|SetMoovingTimerHandler _returnvalue))

(event Custom|IsMoving
  (Pawn|Input|AddMovementInput (Math|Vector|GetUnitDirection(Vector) (Transformation|GetActorLocation) (Variables|Default|GetTragetLocation)) (Variables|Default|GetProbeSpeed) false))

(event Custom|ScanTheFish
  (CallFunction|ScanTarget (Transformation|GetDistanceTo self (Variables|Default|GetTargetFish))))

(event EventMoveHere
  (params (MovementLocation :type Vector :default "0, 0, 0"))
  (Variables|Default|SetTragetLocation MovementLocation)
  (CallFunction|StartMoving)
  (CallFunction|TrytoAnalise))

(event EventBeginPlay
  (Pawn|Components|CharacterMovement|SetMovementMode (Variables|Character|GetCharacterMovement) "MOVE_Flying" 0))

(fn ConstructionScript)

(fn ScanTarget
  (params (DistanceToTarget :type Float%20%28double-precision%29))
  (bind _scandisttxt (Variables|Default|GetScanDistTXT))
  (bind _scandisttxt_2 (Variables|Default|GetScanDistTXT))
  (Rendering|Components|TextRender|SetText _scandisttxt (Utilities|Text|ToText(String) (Class|KismetMathLibrary|ToInt64(Float) DistanceToTarget)))
  (Transformation|SetWorldRotation _scandisttxt "0, 0, 0" false false)
  (Transformation|SetWorldRotation (Variables|Default|GetScanDistTXT) (Math|Rotator|FindLookatRotation (Transformation|GetWorldLocation (Variables|Default|GetScanDistTXT)) (Transformation|GetWorldLocation (Variables|/Script/Engine.Actor|GetRootComponent (Game|GetPlayerCameraManager 0)))) false false)
  (if (<= DistanceToTarget (Variables|Default|GetMAXScaningDistance))
    (Rendering|Components|TextRender|SetTextRenderColor _scandisttxt_2 (LocalVariables|GetInRangeColor%28local%29))
    (Game|Damage|ApplyDamage (Variables|Default|GetTargetFish) (Variables|Default|GetProbe%20Power) 0 self)
    (else
      (Rendering|Components|TextRender|SetTextRenderColor _scandisttxt_2 (LocalVariables|GetOutOfRangeColor%28local%29)))))