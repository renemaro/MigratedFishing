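; Fish pawn that reacts to a nearby probe through a state machine, with debug prints throughout.
; Looping timers drive each behavior: idle scans within a sense radius, cautious drains a fear meter faster at closer range, and recover refills it.
; When fear modulo 100 runs low, a brief timed swim toward an arrow-derived target fires, then returns to idle.
; Zero fear enters Fear, which, like the Dash state, only prints.
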(event Custom|ChangeState
  (params (State :type EN_FishStates%20Enum :default "NewEnumerator0"))
  (switch Utilities|FlowControl|Switch|SwitchonEN_FishStates State
    (:NewEnumerator0
      (Development|PrintString "IDLE" true true "(R=1.000000,G=0.000000,B=0.847957,A=1.000000)" 4.0)
      (CallFunction|ScanforProbe))
    (:NewEnumerator1
      (Development|PrintString "CAUTIOUS" true true "(R=1.000000,G=0.000000,B=0.847957,A=1.000000)" 4.0)
      (CallFunction|Caotious))
    (:NewEnumerator3
      (Development|PrintString "RECOVER" true true "(R=1.000000,G=0.000000,B=0.847957,A=1.000000)" 4.0)
      (CallFunction|BeginRecover))
    (:NewEnumerator2
      (Development|PrintString "FEAR" true true "(R=1.000000,G=0.000000,B=0.847957,A=1.000000)" 4.0))
    (:NewEnumerator4
      (Development|PrintString "DASH" true true "(R=1.000000,G=0.000000,B=0.847957,A=1.000000)" 4.0))))

(event Custom|IdleState
  (bind _returnvalue (Utilities|Time|SetTimerbyEvent 0 0.01))
  (Variables|Default|SetIdleStaeHandler _returnvalue))

(event Custom|Scanning
  (bind _inrange (CallFunction|ScanAreaforProbeF))
  (if _inrange
    (CallFunction|ChangeState "NewEnumerator1")
    (Utilities|Time|ClearandInvalidateTimerbyHandle (Variables|Default|GetIdleScanningHandler))))

(event Custom|ScanForProbe
  (Variables|Default|GetProbe%20Ref
    (:then
      (bind _returnvalue (Utilities|Time|SetTimerbyEvent (delegate Custom|Scanning) 0.01 true))
      (Variables|Default|SetIdleScanningHandler _returnvalue))
    (:else)))

(event Custom|Caotious
  (bind _returnvalue (Utilities|Time|SetTimerbyFunctionName 0 "AnalizeProbe_F" 0.01 true))
  (Variables|Default|SetCaotiousHandler _returnvalue))

(event Custom|BeginRecover
  (bind _returnvalue (Utilities|Time|SetTimerbyFunctionName 0 "Recover_F" 0.01 true))
  (Variables|Default|SetRecoverHandler _returnvalue))

(event Custom|DashFromProbe
  (Variables|Default|SetTragetLocation (+ (Math|Vector|GetForwardVector (Transformation|GetWorldRotation (Variables|Default|GetDirectionArrow))) (Math|Conversions|ToVector(Float) 2e+02)))
  (CallFunction|ActivateSwiming)
  (Utilities|FlowControl|Delay 0.3)
  (Utilities|Time|ClearandInvalidateTimerbyHandle (Variables|Default|GetDashFromProbeHandler))
  (CallFunction|ChangeState "NewEnumerator0"))

(event Custom|Swim
  (CallFunction|SwimF 0.5))

(event Custom|ActivateSwiming
  (bind _returnvalue (Utilities|Time|SetTimerbyEvent (delegate Custom|Swim) 0.01 true))
  (Variables|Default|SetDashFromProbeHandler _returnvalue))

(event EventBeginPlay
  (CallFunction|ChangeState "NewEnumerator0"))

(event EventSetFishState
  (params (State :type EN_FishStates%20Enum :default "NewEnumerator0"))
  (CallFunction|ChangeState State))

(event EventProbeIsActive
  (params (ProbeRef :type BP%20Scanner%20Probe%20Object%20Reference))
  (Variables|Default|SetProbe%20Ref ProbeRef)
  (CallFunction|ScanforProbe))

(fn ConstructionScript)

(fn ScanAreaforProbeF
  (return (<= (Transformation|GetDistanceTo (Variables|Default|GetProbe%20Ref)) (Variables|Default|GetSenceRadius))))

(fn AnalizeProbeF
  (bind _probe_ref (Variables|Default|GetProbe%20Ref))
  (bind _returnvalue (Transformation|GetDistanceTo _probe_ref))
  (if (< _returnvalue (Variables|Default|GetSenceRadius))
    (bind _output_get (Variables|Default|SetCurrentFear (- (Variables|Default|GetCurrentFear) (/ (Variables|Default|GetSenceRadius) _returnvalue))))
    (if (<= _output_get 0.0)
      (Utilities|Time|ClearandInvalidateTimerbyHandle (Variables|Default|GetCaotiousHandler))
      (CallFunction|ChangeState "NewEnumerator2")
      (else
        (Development|PrintString (Utilities|String|ToString(Float) (.Remainder (Math|Float|Division(WholeandRemainder) _output_get 1e+02))) true true "(R=0.119440,G=0.000000,B=1.000000,A=1.000000)")
        (if (<= (.Remainder (Math|Float|Division(WholeandRemainder) _output_get 1e+02)) 1e+01)
          (CallFunction|DashfromProbe))))
    (else
      (Utilities|Time|ClearandInvalidateTimerbyHandle (Variables|Default|GetCaotiousHandler))
      (CallFunction|ChangeState "NewEnumerator3"))))

(fn RecoverF
  (if (>= (Variables|Default|GetCurrentFear) (Variables|Default|GetMaxFear))
    (Utilities|Time|ClearandInvalidateTimerbyHandle (Variables|Default|GetRecoverHandler))
    (Variables|Default|SetCurrentFear (Variables|Default|GetMaxFear))
    (CallFunction|ChangeState "NewEnumerator0")
    (else
      (bind _output_get (Variables|Default|SetCurrentFear (+ (Variables|Default|GetCurrentFear) (Variables|Default|GetRecoverAmmount))))
      (Development|PrintString (Utilities|String|ToString(Float) _output_get) true true "(R=0.242466,G=1.000000,B=0.000000,A=1.000000)"))))

(fn SwimF
  (params (Speed :type Float%20%28single-precision%29))
  (Pawn|Input|AddMovementInput (Math|Vector|GetUnitDirection(Vector) (Transformation|GetActorLocation) (Variables|Default|GetTragetLocation)) Speed false))