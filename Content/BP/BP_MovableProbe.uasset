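; BP_MovableProbe is a flying character probe that travels toward a given location and destroys any overlapping actor tagged Fish.
; MoveHere stores the target location and starts a fast looping timer that repeatedly adds scaled movement input toward it.
; The graph has no arrival check and never clears the timer, so the input keeps being applied once movement starts.
; The capsule's begin-overlap event handles the Fish destruction.
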(event OnComponentBeginOverlap(Capsule)
  (params (OverlappedComponent :type Primitive%20Component%20Object%20Reference) (OtherActor :type Actor%20Object%20Reference) (OtherComp :type Primitive%20Component%20Object%20Reference) (OtherBodyIndex :type Integer) (bFromSweep :type Boolean) (SweepResult :type Hit%20Result%20Structure%20%28by%20ref%29))
  (if (Actor|ActorHasTag OtherActor "Fish")
    (Actor|DestroyActor OtherActor)))

(event Custom|StartMoving
  (bind _returnvalue (Utilities|Time|SetTimerbyEvent (delegate Custom|IsMoving) 0.01 true))
  (Variables|Default|SetMoovingTimerHandler _returnvalue))

(event Custom|IsMoving
  (Pawn|Input|AddMovementInput (Math|Vector|GetUnitDirection(Vector) (Transformation|GetActorLocation) (Variables|Default|GetTragetLocation)) 0.3 false))

(event EventMoveHere
  (params (MovementLocation :type Vector :default "0, 0, 0"))
  (Variables|Default|SetTragetLocation MovementLocation)
  (CallFunction|StartMoving))

(event EventBeginPlay
  (Pawn|Components|CharacterMovement|SetMovementMode (Variables|Character|GetCharacterMovement) "MOVE_Flying" 0))

(fn ConstructionScript)